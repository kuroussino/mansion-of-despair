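; Player character with Enhanced Input movement and look, crosshair-based interaction and a talking mode.
; Each tick outside conversation, a camera ray tracks the watched interactable and grows or shrinks the HUD crosshair.
; Interact input dispatches through collectible, talkable and openable interface checks, though openables cast directly to BP_Door, as does the separate open-door input.
; BeginTalking and StopTalking toggle movement, camera zoom, look sensitivity and crosshair visibility.
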(event Input|EnhancedActionEvents|EnhancedInputActionIA_Move
  (params (ActionValue :type Vector%202D%20Structure) (ElapsedSeconds :type Float%20%28double-precision%29) (TriggeredSeconds :type Float%20%28double-precision%29) (InputAction :type Input%20Action%20Object%20Reference :default "/Game/Core/Inputs/Actions/IA_Move.IA_Move"))
  (bind _returnvalue (Pawn|GetControlRotation :!class /Script/Engine.Pawn))
  (bind (_x _y) (Math|Vector2D|BreakVector2D ActionValue))
  ;[0.8627 0.7451 0.06667] Move
  (Pawn|Input|AddMovementInput (Math|Vector|GetRightVector (Math|Rotator|MakeRotator (.roll _returnvalue) 0.0 (.yaw _returnvalue))) _x false) ; X
  (Pawn|Input|AddMovementInput (Math|Vector|GetForwardVector (Math|Rotator|MakeRotator 0.0 0.0 (.yaw (Pawn|GetControlRotation :!class /Script/Engine.Pawn)))) _y false) ; Y
)

(event Input|EnhancedActionEvents|EnhancedInputActionIA_Look
  (params (ActionValue :type Vector%202D%20Structure) (ElapsedSeconds :type Float%20%28double-precision%29) (TriggeredSeconds :type Float%20%28double-precision%29) (InputAction :type Input%20Action%20Object%20Reference :default "/Game/Core/Inputs/Actions/IA_Look.IA_Look"))
  (bind (_x _y) (Math|Vector2D|BreakVector2D ActionValue))
  ;[0.8627 0.7451 0.06667] Look
  (Pawn|Input|AddControllerYawInput (* _x (Variables|Default|GetcameraRotationMultiplier)))
  (Pawn|Input|AddControllerPitchInput (* _y (Variables|Default|GetcameraRotationMultiplier))))

(event Input|EnhancedActionEvents|EnhancedInputActionIA_Interact
  (params (ActionValue :type Boolean) (ElapsedSeconds :type Float%20%28double-precision%29) (TriggeredSeconds :type Float%20%28double-precision%29) (InputAction :type Input%20Action%20Object%20Reference :default "/Game/Core/Inputs/Actions/IA_Interact.IA_Interact"))
  (bind _currentwatchedinteractable (Variables|Default|GetcurrentWatchedInteractable))
  (bind _currentwatchedinteractable_2 (Variables|Default|GetcurrentWatchedInteractable))
  (bind _currentwatchedinteractable_3 (Variables|Default|GetcurrentWatchedInteractable))
  (:Started
    (Utilities|IsValid (Variables|Default|GetcurrentWatchedInteractable)
      (:Is%20Valid
        (Utilities|FlowControl|Sequence
          (:then_0
            (if (Utilities|DoesObjectImplementInterface _currentwatchedinteractable_3 "/Game/Core/Interactables/BPI_Collectible.BPI_Collectible_C")
              (bind _asbpi_collectible (Utilities|Casting|CastToBPI_Collectible _currentwatchedinteractable_3))
              (Default|Collect _asbpi_collectible)))
          (:then_1
            (if (Utilities|DoesObjectImplementInterface _currentwatchedinteractable_2 "/Game/Core/Interactables/BPI_Talkable.BPI_Talkable_C")
              (bind _asbpi_talkable (Utilities|Casting|CastToBPI_Talkable _currentwatchedinteractable_2))
              (Default|Talk _asbpi_talkable)))
          (:then_2
            (if (Utilities|DoesObjectImplementInterface _currentwatchedinteractable "/Game/Core/Interactables/BPI_Openable.BPI_Openable_C")
              (bind _asbp_door (Utilities|Casting|CastToBP_Door _currentwatchedinteractable))
              (Default|Interact _asbp_door))))))))

(event Input|EnhancedActionEvents|EnhancedInputActionIA_OpenDoor
  (params (ActionValue :type Boolean) (ElapsedSeconds :type Float%20%28double-precision%29) (TriggeredSeconds :type Float%20%28double-precision%29) (InputAction :type Input%20Action%20Object%20Reference :default "/Game/Core/Inputs/Actions/IA_OpenDoor.IA_OpenDoor"))
  (bind _currentwatchedinteractable (Variables|Default|GetcurrentWatchedInteractable))
  (:Completed
    (Utilities|IsValid (Variables|Default|GetcurrentWatchedInteractable)
      (:Is%20Valid
        (if (Utilities|DoesObjectImplementInterface _currentwatchedinteractable "/Game/Core/Interactables/BPI_Openable.BPI_Openable_C")
          (bind _asbp_door (Utilities|Casting|CastToBP_Door _currentwatchedinteractable))
          (Default|Open _asbp_door))))))

(event EventBeginPlay
  ;[0.8627 0.7451 0.06667] EIAS Initialization
  (Utilities|InitializeEIAS
    (:out
      (Utilities|InitializeWidget "/Game/Core/UI/W_MainHUD.W_MainHUD_C"))))

(event EventTick
  (params (DeltaSeconds :type Float%20%28single-precision%29))
  (bind _currentwidget (Variables|Default|GetcurrentWidget))
  (bind _currentwidget_2 (Variables|Default|GetcurrentWidget))
  (if (not (Variables|Default|Gettalking))
    (bind _hitactor (Utilities|TryInteract (Variables|Default|GetPlayerCamera) (Variables|Default|GetinteractRange))
      (:true
        (Utilities|CheckifSameActor _hitactor (Variables|Default|GetcurrentWatchedInteractable)
          (:false
            (Utilities|IsValid _currentwidget
              (:Is%20Valid
                (bind _asw_main_hud (Utilities|Casting|CastToW_MainHUD _currentwidget))
                (Default|GrowCrosshair _asw_main_hud)
                (Variables|Default|SetcurrentWatchedInteractable _hitactor))))))
      (:false
        (Utilities|IsValid (Variables|Default|GetcurrentWatchedInteractable)
          (:Is%20Valid
            (Utilities|IsValid _currentwidget_2
              (:Is%20Valid
                (bind _asw_main_hud_2 (Utilities|Casting|CastToW_MainHUD _currentwidget_2))
                (Default|ShrinkCrosshair _asw_main_hud_2)
                (Variables|Default|SetcurrentWatchedInteractable 0)))))))))

(fn ConstructionScript)

(fn BeginTalking
  (if (not (Variables|Default|Gettalking))
    (Variables|Default|Settalking true)
    (Pawn|Components|CharacterMovement|DisableMovement (Variables|Character|GetCharacterMovement))
    (Camera|SetFieldOfView (Variables|Default|GetPlayerCamera) 5e+01)
    (Variables|Default|SetcameraRotationMultiplier 0.1)
    (bind _asw_main_hud (Utilities|Casting|CastToW_MainHUD (Variables|Default|GetcurrentWidget)))
    (Default|ToggleCrosshair _asw_main_hud false)))

(fn StopTalking
  (if (Variables|Default|Gettalking)
    (Variables|Default|Settalking false)
    (Pawn|Components|CharacterMovement|SetMovementMode (Variables|Character|GetCharacterMovement) "MOVE_Walking" 0)
    (Camera|SetFieldOfView (Variables|Default|GetPlayerCamera) 7e+01)
    (Variables|Default|SetcameraRotationMultiplier 1.0)
    (bind _asw_main_hud (Utilities|Casting|CastToW_MainHUD (Variables|Default|GetcurrentWidget)))
    (Default|ToggleCrosshair _asw_main_hud true)))