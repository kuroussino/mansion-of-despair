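; BP_Ghost is a dialogue NPC that starts hidden and non-collidable, with ToggleVisibility switching both states.
; Each Talk call advances a W_DialogueBox and puts BP_MainCharacter in talking state, while a once-per-conversation timeline turns the player's view toward FocusPosition.
; The first conversation uses per-line speakers, then restores the ghost's BeginPlay location and rotation; later ones show idle lines under NpcName.
; Interact only prints a debug string.
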(event EventInteract
  (Development|PrintString "Interacted"))

(event EventTalk
  (bind _returnvalue (Game|GetPlayerCharacter 0))
  (bind _postdialogueposition (Variables|Default|GetpostDialoguePosition))
  (Utilities|FlowControl|Sequence
    (:then_0
      (Utilities|FlowControl|DoOnce false :!label _label
        (:Completed
          (Components|Timeline|SetPlayRate (Variables|Default|GetFocusOnSpeaker) (/ 1.0 1.0))
          (Timeline|FocusOnSpeaker PlayFromStart
            (:Update
              (Pawn|SetControlRotation (Game|GetPlayerController 0) (Math|Interpolation|RInterpTo (Pawn|GetControlRotation _returnvalue :!class /Script/Engine.Pawn) (Math|Rotator|FindLookatRotation (Transformation|GetActorLocation _returnvalue) (Transformation|GetWorldLocation (Variables|Default|GetFocusPosition))) (Utilities|Time|GetWorldDeltaSeconds) 2.0)))))))
    (:then_1
      (if (Variables|Default|GetalreadyTalkedTo)
        (Math|Integer|IncrementInt (Variables|Default|GetdialogueIndex)
          (:%20%20
            (if (< (Variables|Default|GetdialogueIndex) (Utilities|Array|Length (Variables|Default|GetidleDialogueLines)))
              (bind _asbp_main_character (Utilities|Casting|CastToBP_MainCharacter (Game|GetPlayerCharacter 0)))
              (Default|BeginTalking _asbp_main_character)
              (bind _dialoguewidget (Variables|Default|GetdialogueWidget)
                (:then
                  (Default|SetText _dialoguewidget (Variables|Default|GetnpcName) (Utilities|Array|Get(acopy) (Variables|Default|GetidleDialogueLines) (Variables|Default|GetdialogueIndex))))
                (:else
                  (bind _returnvalue_2 (UserInterface|CreateWidget "/Game/Core/UI/W_DialogueBox.W_DialogueBox_C" (Game|GetPlayerController 0)))
                  (bind _output_get (Variables|Default|SetdialogueWidget _returnvalue_2))
                  (UserInterface|Viewport|AddtoViewport _returnvalue_2 0)
                  (Default|SetText _output_get (Variables|Default|GetnpcName) (Utilities|Array|Get(acopy) (Variables|Default|GetidleDialogueLines) (Variables|Default|GetdialogueIndex)))))
              (else
                (Widget|RemovefromParent (Variables|Default|GetdialogueWidget))
                (bind _asbp_main_character_2 (Utilities|Casting|CastToBP_MainCharacter (Game|GetPlayerCharacter 0)))
                (Default|StopTalking _asbp_main_character_2)
                (Variables|Default|SetdialogueIndex -1)
                (Variables|Default|SetdialogueWidget 0)
                (goto _label Reset)))))
        (else
          (Math|Integer|IncrementInt (Variables|Default|GetdialogueIndex)
            (:%20%20
              (if (< (Variables|Default|GetdialogueIndex) (Utilities|Array|Length (Variables|Default|GetdialogueLines)))
                (bind _asbp_main_character_3 (Utilities|Casting|CastToBP_MainCharacter (Game|GetPlayerCharacter 0)))
                (Default|BeginTalking _asbp_main_character_3)
                (bind _dialoguewidget_2 (Variables|Default|GetdialogueWidget)
                  (:then
                    (Default|SetText _dialoguewidget_2 (Utilities|Array|Get(acopy) (Variables|Default|Getspeakers) (Variables|Default|GetdialogueIndex)) (Utilities|Array|Get(acopy) (Variables|Default|GetdialogueLines) (Variables|Default|GetdialogueIndex))))
                  (:else
                    (bind _returnvalue_3 (UserInterface|CreateWidget "/Game/Core/UI/W_DialogueBox.W_DialogueBox_C" (Game|GetPlayerController 0)))
                    (bind _output_get_2 (Variables|Default|SetdialogueWidget _returnvalue_3))
                    (UserInterface|Viewport|AddtoViewport _returnvalue_3 0)
                    (Default|SetText _output_get_2 (Utilities|Array|Get(acopy) (Variables|Default|Getspeakers) (Variables|Default|GetdialogueIndex)) (Utilities|Array|Get(acopy) (Variables|Default|GetdialogueLines) (Variables|Default|GetdialogueIndex)))))
                (else
                  (Widget|RemovefromParent (Variables|Default|GetdialogueWidget))
                  (bind _asbp_main_character_4 (Utilities|Casting|CastToBP_MainCharacter (Game|GetPlayerCharacter 0)))
                  (Default|StopTalking _asbp_main_character_4)
                  (Variables|Default|SetdialogueIndex -1)
                  (Transformation|SetActorLocationAndRotation (.location _postdialogueposition) (.rotation _postdialogueposition))
                  (Variables|Default|SetalreadyTalkedTo true)
                  (Variables|Default|SetdialogueWidget 0)
                  (goto _label Reset))))))))))

(event EventBeginPlay
  (Variables|Default|SetpostDialoguePosition (Transformation|GetActorTransform))
  (CallFunction|ToggleVisibility false))

(fn ConstructionScript)

(fn ToggleVisibility
  (params (On/Off :type Boolean))
  (if On/Off
    (Rendering|SetVisibility (Variables|Default|GetSkeletalMesh) true false)
    (Collision|SetCollisionEnabled (Variables|Default|GetSkeletalMesh) "QueryAndPhysics")
    (else
      (Rendering|SetVisibility (Variables|Default|GetSkeletalMesh) false false)
      (Collision|SetCollisionEnabled (Variables|Default|GetSkeletalMesh) "NoCollision"))))