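; BP_Door is a door actor that swings its static mesh open.
; The Open event plays the DoorOpening timeline from the start, lerping the mesh's relative yaw from closed to a quarter turn.
; Timeline play rate is the inverse of OpeningTime, so that variable controls the swing duration.
; Interact only prints a debug message and does not trigger Open; no closing logic exists.
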(event EventBeginPlay)

(event Collision|EventActorBeginOverlap
  (params (OtherActor :type Actor%20Object%20Reference)))

(event EventTick
  (params (DeltaSeconds :type Float%20%28single-precision%29)))

(event EventInteract
  (Development|PrintString "door interacted"))

(event EventOpen
  (Development|PrintString "door opened")
  (Components|Timeline|SetPlayRate (Variables|Default|GetDoorOpening) (/ 1.0 (Variables|Default|GetopeningTime)))
  (bind _0_1 (Timeline|DoorOpening PlayFromStart)
    (:Update
      (Transformation|SetRelativeRotation (Variables|Default|GetStaticMesh) (Math|Rotator|MakeRotator 0.0 0.0 (Math|Float|Lerp 0.0 9e+01 _0_1)) false false))))

(fn ConstructionScript)